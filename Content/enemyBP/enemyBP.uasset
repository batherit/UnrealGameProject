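; Enemy actor that damages the hero on contact and destroys itself when its own HP runs out.
; Overlapping a HeroBP sends a damage message at once, then repeats it on a short looping timer until the overlap ends.
; DecreaseHP subtracts incoming damage from the enemy's HP, though both the starting HP and the damage sent to the hero are set to zero here.
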(event Custom|DecreaseHeroHP
  (Class|Damage|DecreaseHP(Message) (stale Collision|EventActorBeginOverlap _ashero_bp) 0.0))

(event EventBeginPlay
  (Variables|Default|SetHP 0.0))

(event Collision|EventActorBeginOverlap
  (params (OtherActor :type Actor%20Object%20Reference))
  (bind _ashero_bp (Utilities|Casting|CastToHeroBP OtherActor))
  (CallFunction|DecreaseHeroHP)
  (Utilities|Time|SetTimerbyFunctionName 0 "DecreaseHeroHP" 0.33 true))

(event EventTick
  (params (DeltaSeconds :type Float%20%28single-precision%29)))

(event EventDecreaseHP
  (params (amount :type Float%20%28single-precision%29))
  (bind _output_get (Variables|Default|SetHP (- (Variables|Default|GetHP) amount)))
  (if (<= _output_get 0.0)
    (Actor|DestroyActor)))

(event Collision|EventActorEndOverlap
  (params (OtherActor :type Actor%20Object%20Reference))
  (Utilities|Casting|CastToHeroBP OtherActor)
  (Utilities|Time|ClearTimerbyFunctionName 0 "DecreaseHeroHP"))

(fn ConstructionScript)